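; BP_Canon is an enemy projectile that damages the player's BP_HeadCharacter on overlap.
; Tick finds the head once, caches the normalized direction to it, then sweeps straight along X and Y without homing.
; Overlapping the head subtracts Health through a DoOnce and destroys the projectile, while BP_RootCharacter only destroys it.
; A BeginPlay timer destroys it after its lifetime, and a BP_BasicEnemy damage branch is left unconnected.
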(event Custom|Destroy
  (Actor|DestroyActor))

(event Custom|DealDamage
  (params (Target :type BP%20Entity%20Object%20Reference))
  (Utilities|FlowControl|DoOnce false
    (:Completed
      (Variables|/Game/FrazierContent/BP_Entity.BP_Entity_C|SetHealth Target (- (Variables|/Game/FrazierContent/BP_Entity.BP_Entity_C|GetHealth Target) (Variables|Default|GetDamage))))))

(event EventTick
  (params (DeltaSeconds :type Float%20%28single-precision%29))
  (Utilities|IsValid (Variables|Default|GetHead)
    (:Is%20Valid
      (Transformation|AddActorWorldOffset (Math|Vector|MakeVector (.x (* (Variables|Default|GetLocation) (Variables|Default|GetSpeed))) (.y (* (Variables|Default|GetLocation) (Variables|Default|GetSpeed))) 0.0) true))
    (:Is%20Not%20Valid
      (bind _returnvalue (Actor|GetActorOfClass "/Game/FrazierContent/Head/BP_HeadCharacter.BP_HeadCharacter_C"))
      (Variables|Default|SetHead _returnvalue)
      (Variables|Default|SetLocation (Math|Vector|Normalize (- (Transformation|GetActorLocation (Variables|Default|GetHead)) (Transformation|GetActorLocation)))))))

(event Collision|EventActorBeginOverlap
  (params (OtherActor :type Actor%20Object%20Reference))
  (bind _asbp_head_character (Utilities|Casting|CastToBP_HeadCharacter OtherActor)
    (:then
      (CallFunction|DealDamage _asbp_head_character))
    (:CastFailed
      (Utilities|Casting|CastToBP_RootCharacter OtherActor)))
  (CallFunction|Destroy))

(event EventBeginPlay
  (Utilities|Time|SetTimerbyEvent (delegate Custom|Destroy) (Variables|Default|GetTimeTillAutoDestroy)))

(fn ConstructionScript)