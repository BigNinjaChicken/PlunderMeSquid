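; Player root character that moves relative to its camera, bobs its mesh, spawns a tentacle and grabs or throws enemies.
; Grab input passes a timeline-driven cooldown gate, then sphere-overlaps ahead to attach a BP_RootEnemy or launches the held one forward.
; Tick applies movement toward BP_HeadCharacter when beyond a maximum radius.
; The detached camera boom follows the Head, scaling its offset with the farthest player's distance from it.
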(event Custom|MeshBobb
  (Components|Timeline|SetPlayRate (Variables|Default|GetT_Bobb) 0.4)
  (bind _value (Timeline|T_Bobb PlayFromStart)
    (:Update
      (Transformation|SetRelativeLocation (Variables|Character|GetMesh) (Math|Vector|MakeVector 0.0 0.0 (Math|Float|Lerp -9e+01 -6e+01 _value)) false false))
    (:Finished
      (Timeline|T_Bobb PlayFromStart))))

(event Custom|PlayerInput%20Move
  (params (X :type Float%20%28double-precision%29) (Y :type Float%20%28double-precision%29))
  (bind _followcamera (Variables|Camera|GetFollowCamera))
  (bind _returnvalue (Transformation|GetWorldRotation _followcamera))
  (Pawn|Input|AddMovementInput (Math|Vector|GetRightVector (Math|Rotator|MakeRotator (.roll _returnvalue) 0.0 (.yaw _returnvalue))) X false)
  (Pawn|Input|AddMovementInput (Math|Vector|GetForwardVector (Math|Rotator|MakeRotator 0.0 0.0 (.yaw (Transformation|GetWorldRotation _followcamera)))) Y false))

(event Custom|PlayerInput%20Grab
  (bind _returnvalue (Transformation|GetActorLocation))
  (bind _returnvalue_2 (Transformation|GetActorForwardVector))
  (bind _returnvalue_3 (Transformation|GetActorForwardVector))
  (bind _force (Variables|Grab|GetForce))
  (bind _grabhitboxdistance (Variables|Grab|GetGrabHitBoxDistance))
  (bind _sphereradius (Variables|Grab|GetSphereRadius))
  (bind _returnvalue_4 (* _returnvalue_3 _force))
  (bind _returnvalue_5 (* _returnvalue_2 _grabhitboxdistance))
  (bind _returnvalue_6 (+ _returnvalue _returnvalue_5))
  (Utilities|FlowControl|Gate false
    (:Exit
      (if (Variables|Grab|GetHasPickedUpEnemy)
        (CallFunction|GrabCooldown 2.0)
        (Transformation|DetachFromActor (Variables|Grab|GetPickedUpEnemy) "KeepWorld" "KeepWorld" "KeepWorld")
        (Variables|/Script/Engine.MovementComponent|SetVelocity (Variables|/Script/Engine.Character|GetCharacterMovement (Variables|Grab|GetPickedUpEnemy)) (Math|Vector|MakeVector (.x _returnvalue_4) (.y _returnvalue_4) 0.0))
        (Variables|/Game/FrazierContent/Enemy/BP_RootEnemy.BP_RootEnemy_C|SetReady (Variables|Grab|GetPickedUpEnemy) true)
        (Utilities|Time|SetTimerbyEvent (delegate Custom|AddBackCollsion) 2.0)
        (Variables|Grab|SetHasPickedUpEnemy false)
        (else
          (CallFunction|GrabCooldown 2.0)
          (bind _outactors (Collision|SphereOverlapActors _returnvalue_6 _sphereradius (Variables|Grab|GetObject%20Types) 0))
          (Rendering|Debug|DrawDebugSphere _returnvalue_6 _sphereradius 12 "(R=1.000000,G=0.000000,B=0.073746,A=1.000000)" 0.1 2.0)
          (for _array_element _outactors
            (bind _asbp_root_enemy (Utilities|Casting|CastToBP_RootEnemy _array_element))
            (Variables|Grab|SetPickedUpEnemy _asbp_root_enemy)
            (Variables|Grab|SetHasPickedUpEnemy true)
            (CallFunction|PickUpEnemy)))))))

(event Custom|PickUpEnemy
  (bind _pickedupenemy (Variables|Grab|GetPickedUpEnemy))
  (CallFunction|GrabCooldown 1.0)
  (Variables|/Game/FrazierContent/Enemy/BP_RootEnemy.BP_RootEnemy_C|SetReady (Variables|Grab|GetPickedUpEnemy) false)
  (Collision|SetCollisionResponsetoChannel (Variables|Default|GetCapsuleComponent) "ECC_GameTraceChannel1" "ECR_Overlap")
  (Transformation|AttachActorToActor _pickedupenemy self "Bone_006" "SnapToTarget" "KeepWorld" "KeepWorld" true)
  (Transformation|SetActorLocation _pickedupenemy (+ (* (Transformation|GetActorForwardVector) (Variables|Grab|GetGrabHitBoxDistance)) (Transformation|GetActorLocation)) false false))

(event Custom|GrabCooldown
  (params (Duration :type Float%20%28double-precision%29))
  (bind _returnvalue (Transformation|GetActorLocation))
  (bind _returnvalue_2 (Transformation|GetActorForwardVector))
  (bind _returnvalue_3 (Transformation|GetActorForwardVector))
  (bind _force (Variables|Grab|GetForce))
  (bind _grabhitboxdistance (Variables|Grab|GetGrabHitBoxDistance))
  (bind _sphereradius (Variables|Grab|GetSphereRadius))
  (bind _returnvalue_4 (* _returnvalue_3 _force))
  (bind _returnvalue_5 (* _returnvalue_2 _grabhitboxdistance))
  (bind _returnvalue_6 (+ _returnvalue _returnvalue_5))
  (Components|Timeline|SetPlayRate (Variables|Default|GetT_Cooldown) (/ 1.0 Duration))
  (Timeline|T_Cooldown PlayFromStart
    (:Update
      (Utilities|FlowControl|Gate false) ; enters at Close
    )
    (:Finished
      (Utilities|FlowControl|Gate false) ; enters at Open
    )))

(event Custom|AddBackCollsion
  (Collision|SetCollisionResponsetoChannel (Variables|Default|GetCapsuleComponent) "ECC_GameTraceChannel1" "ECR_Block"))

(event EventBeginPlay
  (Utilities|FlowControl|Sequence
    (:then_0
      (Transformation|DetachFromComponent (Variables|Camera|GetCameraBoom) "KeepWorld" "KeepWorld" "KeepWorld" true))
    (:then_1
      (CallFunction|MeshBobb))
    (:then_2
      (Game|SpawnActorfromClass "/Game/FrazierContent/PC_Tentacle.PC_Tentacle_C" (Transformation|GetActorTransform) "Undefined" 0 0))
    (:then_3
      (bind _asplayer_controller (Utilities|Casting|CastToPlayerController (Pawn|GetController)))
      (Utilities|IsValid (PlayerController|LocalPlayerSubsystems|GetEnhancedInputLocalPlayerSubsystem _asplayer_controller)
        (:Is%20Valid
          (Input|AddMappingContext (PlayerController|LocalPlayerSubsystems|GetEnhancedInputLocalPlayerSubsystem _asplayer_controller) "/Game/FrazierContent/Input/IMC_Player.IMC_Player" 0 "(bIgnoreAllPressedKeysUntilRelease=True,bForceImmediately=False)"))))))

(event EventTick
  (params (DeltaSeconds :type Float%20%28single-precision%29))
  (Utilities|FlowControl|Sequence
    (:then_0
      (if (not (Utilities|IsValid (Variables|Default|GetHead)))
        (bind _returnvalue (Actor|GetActorOfClass "/Game/FrazierContent/Head/BP_HeadCharacter.BP_HeadCharacter_C"))
        (Variables|Default|SetHead _returnvalue)
        (else
          (Utilities|FlowControl|Sequence
            (:then_0
              (if (> (Math|Vector|Distance(Vector) (Transformation|GetActorLocation (Variables|Default|GetHead)) (Transformation|GetActorLocation)) (Variables|Tether|GetMaxRadius))
                (CallFunction|PlayerInputMove (.x (* (Math|Vector|Normalize (Math|Vector|GetUnitDirection(Vector) (Transformation|GetActorLocation) (Transformation|GetActorLocation (Variables|Default|GetHead)))) (Variables|Tether|GetStrength))) (.z (* (Math|Vector|Normalize (Math|Vector|GetUnitDirection(Vector) (Transformation|GetActorLocation) (Transformation|GetActorLocation (Variables|Default|GetHead)))) (Variables|Tether|GetStrength))))))))))
    (:then_2
      (Utilities|IsValid (Variables|Default|GetHead)
        (:Is%20Valid
          (Transformation|SetWorldRotation (Variables|Camera|GetFollowCamera) (Math|Rotator|FindLookatRotation (Transformation|GetWorldLocation (Variables|Camera|GetFollowCamera)) (Transformation|GetWorldLocation (Variables|/Script/Engine.Character|GetCapsuleComponent (Variables|Default|GetHead)))) false false)
          (Transformation|SetWorldLocation (Variables|Camera|GetCameraBoom) (Transformation|GetWorldLocation (Variables|/Script/Engine.Character|GetCapsuleComponent (Variables|Default|GetHead))) false false)
          (bind _greatestdistance (CallFunction|GetFarthestTentacle))
          (Variables|/Script/Engine.SpringArmComponent|SetTargetOffset (Variables|Camera|GetCameraBoom) (Math|Vector|Lerp(Vector) (Variables|Camera|GetMinCamDistance) (Variables|Camera|GetMaxCamDistance) (Math|Float|Clamp(Float) (/ (- _greatestdistance (Variables|Camera|GetMinCamOffset)) (Variables|Camera|GetMaxCamOffset)) 0.65))))))))

(fn ConstructionScript)

(fn GetFarthestTentacle
  (for _array_element (Variables|/Game/FrazierContent/Head/BP_HeadCharacter.BP_HeadCharacter_C|GetAllPlayers (Variables|Default|GetHead))
    (if (> (Transformation|GetDistanceTo _array_element (Variables|Default|GetHead)) (LocalVariables|GetFarthest))
      (bind _output_get (LocalVariables|SetFarthest (Transformation|GetDistanceTo _array_element (Variables|Default|GetHead))))))
  (return _output_get))