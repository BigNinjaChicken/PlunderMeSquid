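; Player 1 character that spawns and drives a two-player setup, with a second root pawn and a Head character between which input and camera are handled.
; BeginPlay adds the input mapping, spawns both actors with default controllers and detaches the camera boom.
; Two move actions steer this pawn and Player 2 from one controller.
; Each tick, the camera tracks the Head, and boom offset scales with distance between the two players.
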(event Input|EnhancedActionEvents|EnhancedInputActionIA_Move2
  (params (ActionValue :type Vector%202D%20Structure) (ElapsedSeconds :type Float%20%28double-precision%29) (TriggeredSeconds :type Float%20%28double-precision%29) (InputAction :type Input%20Action%20Object%20Reference :default "/Game/FrazierContent/Input/IA_Move2.IA_Move2"))
  (:Triggered
    (CallFunction|Move (Variables|Kraken|GetPlayer2) (.x ActionValue) (.y ActionValue))))

(event Input|EnhancedActionEvents|EnhancedInputActionIA_Move1
  (params (ActionValue :type Vector%202D%20Structure) (ElapsedSeconds :type Float%20%28double-precision%29) (TriggeredSeconds :type Float%20%28double-precision%29) (InputAction :type Input%20Action%20Object%20Reference :default "/Game/FrazierContent/Input/IA_Move1.IA_Move1"))
  (:Triggered
    (CallFunction|Move self (.x ActionValue) (.y ActionValue))))

(event EventTick
  (params (DeltaSeconds :type Float%20%28single-precision%29))
  (Utilities|FlowControl|Sequence
    (:then_0
      (Transformation|SetWorldRotation (Variables|Default|GetFollowCamera) (Math|Rotator|FindLookatRotation (Transformation|GetWorldLocation (Variables|Default|GetFollowCamera)) (Transformation|GetWorldLocation (Variables|/Script/Engine.Character|GetCapsuleComponent (Variables|Kraken|GetHead_0)))) false false)
      (Transformation|SetWorldLocation (Variables|Default|GetCameraBoom) (Transformation|GetWorldLocation (Variables|/Script/Engine.Character|GetCapsuleComponent (Variables|Kraken|GetHead_0))) false false)
      (Variables|/Script/Engine.SpringArmComponent|SetTargetOffset (Variables|Default|GetCameraBoom) (Math|Vector|Lerp(Vector) (Variables|Camera|GetMinCamDistance) (Variables|Camera|GetMaxCamDistance) (Math|Float|Clamp(Float) (/ (- (Transformation|GetDistanceTo (Variables|Kraken|GetPlayer2)) (Variables|Camera|GetMinOffset)) (Variables|Camera|GetMaxCamOffset)) 0.3))))))

(event EventBeginPlay
  (bind _capsulecomponent (Variables|Default|GetCapsuleComponent))
  (bind _offset (Variables|Setup|GetOffset))
  (bind _returnvalue (Transformation|GetWorldTransform _capsulecomponent))
  (bind _returnvalue_2 (+ _offset (.y (.location _returnvalue))))
  (bind _returnvalue_3 (+ _offset (.x (.location _returnvalue))))
  (bind _returnvalue_4 (Math|Transform|MakeTransform (Math|Vector|MakeVector _returnvalue_3 _returnvalue_2 (.z (.location _returnvalue))) (.rotation _returnvalue) (.scale _returnvalue)))
  (Utilities|FlowControl|Sequence
    (:then_0
      (bind _asplayer_controller (Utilities|Casting|CastToPlayerController (Pawn|GetController)))
      (Utilities|IsValid (PlayerController|LocalPlayerSubsystems|GetEnhancedInputLocalPlayerSubsystem _asplayer_controller)
        (:Is%20Valid
          (Input|AddMappingContext (PlayerController|LocalPlayerSubsystems|GetEnhancedInputLocalPlayerSubsystem _asplayer_controller) "/Game/FrazierContent/Input/IMC_Player.IMC_Player" 0 "(bIgnoreAllPressedKeysUntilRelease=True,bForceImmediately=False)"))))
    (:then_1
      (bind _returnvalue_5 (Game|SpawnActorfromClass "/Game/FrazierContent/Player/BP_Player2Root.BP_Player2Root_C" _returnvalue_4 "Undefined" 0 0))
      (bind _output_get (Variables|Kraken|SetPlayer2 _returnvalue_5))
      (Pawn|SpawnDefaultController _output_get)
      (bind _returnvalue_6 (Game|SpawnActorfromClass "/Game/FrazierContent/Head/BP_HeadCharacter.BP_HeadCharacter_C" _returnvalue_4 "Undefined" 0 0))
      (Pawn|SpawnDefaultController _returnvalue_6)
      (bind _output_get_2 (Variables|Kraken|SetHead_0 _returnvalue_6))
      (Variables|/Game/FrazierContent/Head/BP_HeadCharacter.BP_HeadCharacter_C|SetReady _output_get_2 true))
    (:then_2
      (Transformation|DetachFromComponent (Variables|Default|GetCameraBoom) "KeepWorld" "KeepWorld" "KeepWorld" true))
    (:then_3
      (CallFunction|MeshBobb))))

(fn ConstructionScript
  (|CallParentFunction))