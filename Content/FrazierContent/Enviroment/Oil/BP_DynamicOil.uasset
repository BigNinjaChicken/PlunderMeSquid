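; BP_DynamicOil is a procedural oil volume that builds a box mesh and cuts holes in it with Geometry Script.
; Its construction script calls CreateBox, which resets the dynamic mesh, appends a box sized by Size and releases pooled compute meshes.
; AddHole rebuilds the box, then boolean-subtracts a cylinder for every BP_CutterOil actor in the level, using its world offset, rotation and scale.
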(event EventBeginPlay)

(event Collision|EventActorBeginOverlap
  (params (OtherActor :type Actor%20Object%20Reference)))

(event EventTick
  (params (DeltaSeconds :type Float%20%28single-precision%29)))

(fn ConstructionScript
  (CallFunction|CreateBox)
  (CallFunction|AddHole))

(fn AddHole
  (bind _outactors (Actor|GetAllActorsOfClass "/Game/FrazierContent/Enviroment/Oil/BP_CutterOil.BP_CutterOil_C"))
  (CallFunction|CreateBox)
  (for _array_element _outactors
    (bind _returnvalue (DynamicMeshActor|AllocateComputeMesh))
    (bind _returnvalue_2 (GeometryScript|Primitives|AppendCylinder :TargetMesh _returnvalue :Transform (Math|Transform|MakeTransform (* (- (.location (Transformation|GetActorTransform)) (.location (Transformation|GetActorTransform _array_element))) -1.0) (.rotation (Transformation|GetActorTransform _array_element)) (.scale (Transformation|GetActorTransform _array_element))) :Radius 6e+01 :RadialSteps 40 :Debug 0))
    (bind _returnvalue_3 (DynamicMeshComponent|GetDynamicMesh (Variables|DynamicMeshActor|GetDynamicMeshComponent)))
    (GeometryScript|Booleans|ApplyMeshBoolean :TargetMesh _returnvalue_3 :ToolMesh _returnvalue_2 :Operation "Subtract" :Debug 0)))

(fn CreateBox
  (bind _size (Variables|Default|GetSize))
  (bind _returnvalue (DynamicMeshComponent|GetDynamicMesh (Variables|DynamicMeshActor|GetDynamicMeshComponent)))
  (bind _returnvalue_2 (DynamicMesh|Reset _returnvalue))
  (Class|GeometryScriptLibraryMeshPrimitiveFunctions|AppendBox :TargetMesh _returnvalue_2 :DimensionX (.x _size) :DimensionY (.y _size) :DimensionZ (.z _size) :StepsX 2 :StepsY 2 :StepsZ 2 :Debug 0)
  (DynamicMeshActor|ReleaseAllComputeMeshes))