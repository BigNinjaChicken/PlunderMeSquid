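; BP_DangerSpline is an environment actor that generates a flat ribbon mesh along an editable spline, with no runtime logic.
; The construction script builds one procedural mesh quad section per pair of neighboring spline points, extending from the spline along each point's right vector by Size.
; Each section receives the Mat_Cannon material.
; UV calculations are left unconnected, so the sections are created without UVs.
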(event EventBeginPlay)

(event Collision|EventActorBeginOverlap
  (params (OtherActor :type Actor%20Object%20Reference)))

(event EventTick
  (params (DeltaSeconds :type Float%20%28single-precision%29)))

(fn ConstructionScript
  (bind _spline (Variables|Default|GetSpline))
  (bind _size (Variables|Default|GetSize))
  (for _index (range 0 (- (Spline|GetNumberOfSplinePoints (Variables|Default|GetSpline)) 2))
    (Variables|Default|SetIndex _index)
    (Variables|Default|SetPoint1Orgin (Spline|GetLocationatSplinePoint _spline _index "Local"))
    (Variables|Default|SetPoint1Extended (+ (Spline|GetLocationatSplinePoint _spline _index "Local") (* (Class|SplineComponent|GetRightVectoratSplinePoint _spline _index "Local") _size)))
    (Variables|Default|SetPoint2Orgin (Spline|GetLocationatSplinePoint _spline (+ _index 1) "Local"))
    (Variables|Default|SetPoint2Extened (+ (Spline|GetLocationatSplinePoint _spline (+ _index 1) "Local") (* (Class|SplineComponent|GetRightVectoratSplinePoint _spline (+ _index 1) "Local") _size)))
    (Class|ProceduralMeshComponent|CreateMeshSectionLinearColor (Variables|Default|GetProceduralMesh) (Variables|Default|GetIndex) (Utilities|Array|MakeArray (Variables|Default|GetPoint1Orgin) (Variables|Default|GetPoint1Extended) (Variables|Default|GetPoint2Orgin) (Variables|Default|GetPoint2Extened)) (Utilities|Array|MakeArray 0 1 2 3 2 1) 0 0 0 0 0 0 0 false false)
    (Rendering|Material|SetMaterial (Variables|Default|GetProceduralMesh) (Variables|Default|GetIndex) "/Game/FrazierContent/Entity/Enemy/RootEnemy/Mat_Cannon.Mat_Cannon")))