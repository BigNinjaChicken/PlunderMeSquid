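; BP_Test is a test Blueprint that prints the name of a pressed input to show which key fired.
; Hard-wired key events for Up, W and the gamepad top face button each pass their key's long display name to Print String.
; It has no other logic, and its construction script is empty.
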(event Input|KeyboardEvents|Up
  (params (Key :type Key%20Structure :default "None"))
  (:Pressed
    (Development|PrintString (Utilities|String|ToString(Text) (Class|KismetInputLibrary|KeyGetDisplayName Key true)))))

(event Input|KeyboardEvents|W
  (params (Key :type Key%20Structure :default "None"))
  (:Pressed
    (Development|PrintString (Utilities|String|ToString(Text) (Class|KismetInputLibrary|KeyGetDisplayName Key true)))))

(event Input|GamepadEvents|GamepadFaceButtonTop
  (params (Key :type Key%20Structure :default "None"))
  (:Pressed
    (Development|PrintString (Utilities|String|ToString(Text) (Class|KismetInputLibrary|KeyGetDisplayName Key true)))))

(fn ConstructionScript)