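; Local multiplayer game mode that creates a player for each tagged PlayerStart in the level.
; On BeginPlay it gathers PlayerStarts and matches their integer-converted tags to player indices.
; Each index gets a local player and a possessed BP_InputReceiver, with receivers and controllers stored in arrays.
; SpawnPlayer later spawns BP_Tentacle3Players at a given receiver's transform and hands possession to that player's controller.
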(event EventBeginPlay
  (CallFunction|GetPlayerStartPoints)
  (CallFunction|SpawnInputReceivers))

(fn ConstructionScript)

(fn GetPlayerStartPoints
  (bind _outactors (Actor|GetAllActorsOfClass "/Script/Engine.PlayerStart"))
  (Variables|Default|SetPlayerStartArray _outactors))

(fn SpawnInputReceivers
  (for (_ _array_index) (Variables|Default|GetPlayerStartArray)
    (LocalVariables|SetIndex _array_index)
    (for _array_element (Variables|Default|GetPlayerStartArray)
      (if (== (CallFunction|NametoInt _array_element) (LocalVariables|GetIndex))
        (bind _returnvalue (Class|GameplayStatics|CreatePlayer (LocalVariables|GetIndex)))
        (bind _returnvalue_2 (Game|SpawnActorfromClass "/Game/FrazierContent/Multiplayer/BP_InputReceiver.BP_InputReceiver_C" (Transformation|GetActorTransform (Utilities|Array|Get(acopy) (Variables|Default|GetPlayerStartArray) (LocalVariables|GetIndex))) "Undefined" _returnvalue (LocalVariables|GetIndex) 0))
        (Utilities|Array|AddUnique (Variables|Default|GetPlayerInputReceiverArray) _returnvalue_2)
        (Pawn|Possess (Game|GetPlayerController (LocalVariables|GetIndex)) _returnvalue_2)
        (Utilities|Array|AddUnique (Variables|Default|GetPlayerControllerArray) (Game|GetPlayerController (LocalVariables|GetIndex)))))))

(fn NametoInt
  (params (PlayerStart :type Player%20Start%20Object%20Reference))
  (return (Math|Conversions|ToInteger(Byte) (Utilities|String|ToString(Name) (Variables|/Script/Engine.PlayerStart|GetPlayerStartTag PlayerStart)))))

(fn SpawnPlayer
  (params (CurrentPlayerIndex :type Integer) (Input%20Receiver :type BP%20Input%20Receiver%20Object%20Reference))
  (bind _returnvalue (Game|SpawnActorfromClass "/Game/FrazierContent/Entity/Player/BP_Tentacle3Players.BP_Tentacle3Players_C" (Transformation|GetActorTransform Input%20Receiver) "Undefined" 0 CurrentPlayerIndex 0))
  (Pawn|Possess (Game|GetPlayerController CurrentPlayerIndex) _returnvalue)
  (return false))