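; BP_RootEnemy is an enemy ship with health, collision damage and a cannon, tracking the BP_HeadCharacter.
; ShootEvent spawns a BP_Canon aimed at the head and restarts the cooldown timeline.
; Hits on solid hazards, root characters or other enemies deal damage, hurting both enemies in enemy collisions.
; On death, bosses open the next stage by incrementing the level name's final digit; others spawn crew, notify GM_StageRoot and destroy themselves.
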(event Custom|ShootEvent
  (bind _selflocation (Variables|Default|GetSelfLocation))
  (bind _headlocation (Variables|Default|GetHeadLocation))
  (bind _selflocation_2 (Variables|Default|GetSelfLocation))
  (bind _returnvalue (Math|Rotator|FindLookatRotation _selflocation _headlocation))
  (bind _returnvalue_2 (Math|Vector|GetForwardVector _returnvalue))
  (bind _returnvalue_3 (* _returnvalue_2 5e+01))
  (bind _returnvalue_4 (+ _returnvalue_3 _selflocation_2))
  (Utilities|FlowControl|Sequence
    (:then_0
      (Components|Timeline|SetPlayRate (Variables|Default|GetCooldown) 0.25)
      (Timeline|Cooldown PlayFromStart
        (:Finished
          (Variables|Default|SetCanShoot true))))
    (:then_1
      (Game|SpawnActorfromClass "/Game/FrazierContent/Entity/Enemies/RootEnemy/BP_Canon.BP_Canon_C" (Math|Transform|MakeTransform (Math|Vector|MakeVector (.x _returnvalue_4) (.y _returnvalue_4) (+ (.z _returnvalue_4) 6e+01)) _returnvalue "1.000000,1.000000,1.000000") "Undefined" 0 0))
    (:then_2
      (Audio|SpawnSoundatLocation "/Game/FrazierContent/Sounds/SW_CannonFire.SW_CannonFire" (Transformation|GetActorLocation) "0, 0, 0" 1.0 1.3 0.0 0 0))))

(event EventTick
  (params (DeltaSeconds :type Float%20%28single-precision%29))
  (|CallParentFunction DeltaSeconds)
  (Utilities|IsValid (Variables|Default|GetHead)
    (:Is%20Valid
      (Utilities|FlowControl|Sequence
        (:then_0
          (Variables|Default|SetSelfLocation (Transformation|GetActorLocation)))
        (:then_1
          (Variables|Default|SetHeadLocation (Transformation|GetActorLocation (Variables|Default|GetHead))))))
    (:Is%20Not%20Valid
      (bind _returnvalue (Actor|GetActorOfClass "/Game/FrazierContent/Entity/Head/BP_HeadCharacter.BP_HeadCharacter_C"))
      (Variables|Default|SetHead _returnvalue))))

(event EventBeginPlay
  (Utilities|FlowControl|Sequence
    (:then_0
      (Variables|Default|SetHealth 1e+01))
    (:then_1
      (Utilities|FlowControl|Delay 0.2)
      (Variables|Default|SetReady true))
    (:then_2
      (bind _returnvalue (Actor|GetActorOfClass "/Game/FrazierContent/Entity/Head/BP_HeadCharacter.BP_HeadCharacter_C"))
      (Variables|Default|SetHead _returnvalue))))

(event EventDeath
  (Utilities|FlowControl|DoOnce false
    (:Completed
      (if (Variables|Default|GetIsBoss)
        (bind _returnvalue (Game|GetCurrentLevelName true))
        (CallFunction|ToNextStage _returnvalue)
        (else
          (for _index (range 0 (- (Variables|Default|GetCrewAmount) 1))
            (Game|SpawnActorfromClass "/Game/FrazierContent/Entity/Enemies/Crew/BP_Crew.BP_Crew_C" (Transformation|GetActorTransform) "Undefined" 0 0))
          (Audio|SpawnSound2D "/Game/FrazierContent/Sounds/SW_Bell.SW_Bell" 1.0 1.0 0.0 0)
          (Audio|SpawnSoundAttached "/Game/FrazierContent/Sounds/SW_ShipBreak.SW_ShipBreak" (Variables|Character|GetMesh) "None" "0, 0, 0" "0, 0, 0" "KeepRelativeOffset" false 1.0 1.0 0.0 0 0)
          (Utilities|FlowControl|Delay 0.2)
          (bind _returnvalue_2 (Actor|GetActorOfClass "/Game/FrazierContent/Stages/Game/GM_StageRoot.GM_StageRoot_C"))
          (Default|UpdateEnemyCount _returnvalue_2) ; Tell GameMode Enemy Died
          (Actor|DestroyActor))))))

(event Collision|EventHit
  (params (MyComp :type Primitive%20Component%20Object%20Reference) (Other :type Actor%20Object%20Reference) (OtherComp :type Primitive%20Component%20Object%20Reference) (bSelfMoved :type Boolean) (HitLocation :type Vector :default "0, 0, 0") (HitNormal :type Vector :default "0, 0, 0") (NormalImpulse :type Vector :default "0, 0, 0") (Hit :type Hit%20Result%20Structure%20%28by%20ref%29))
  (if (Variables|Default|GetCanTakeHitDamage)
    (Utilities|Casting|CastToBP_SoildHazard Other
      (:then
        _)
      (:CastFailed
        (Utilities|Casting|CastToBP_RootCharacter Other
          (:then
            _)
          (:CastFailed
            (bind _asbp_root_enemy (Utilities|Casting|CastToBP_RootEnemy Other))
            (CallFunction|DealDamage _asbp_root_enemy 1e+01)))))
    (CallFunction|DealDamage self 1e+01)))

(fn ConstructionScript)

(fn ToNextStage
  (params (SourceString :type String))
  (bind _returnvalue (Utilities|String|GetCharacterArrayfromString SourceString))
  (bind _returnvalue_2 (Utilities|Array|Length _returnvalue))
  (bind _returnvalue_3 (- _returnvalue_2 1))
  (bind _output (Utilities|Array|Get(acopy) _returnvalue _returnvalue_3))
  (Game|OpenLevel(byName) (Utilities|String|StringToName (Utilities|String|Replace SourceString (Utilities|String|Append "_" _output) (Utilities|String|Append "_" (Utilities|String|ToString(Integer) (+ (Math|Conversions|ToInteger(Byte) _output) 1)))))))