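; BP_Canon is an enemy projectile that damages the player's BP_HeadCharacter on impact.
; Each tick it sweeps along its forward vector in X and Y only, once it has found a head character in the level.
; Hits on that character subtract Damage from Health a single time through a DoOnce and call TakeDamge.
; Any hit destroys the projectile, as does a lifetime timer started on BeginPlay.
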(event Custom|Destroy
  (Actor|DestroyActor))

(event Custom|DealDamage
  (params (Target :type BP%20Entity%20Object%20Reference))
  (Utilities|FlowControl|DoOnce false
    (:Completed
      (Variables|/Game/FrazierContent/Entity/BP_Entity.BP_Entity_C|SetHealth Target (- (Variables|/Game/FrazierContent/Entity/BP_Entity.BP_Entity_C|GetHealth Target) (Variables|Default|GetDamage)))
      (bind _asbp_head_character (Utilities|Casting|CastToBP_HeadCharacter Target))
      (Default|TakeDamge _asbp_head_character))))

(event EventTick
  (params (DeltaSeconds :type Float%20%28single-precision%29))
  (bind _returnvalue (Transformation|GetActorForwardVector))
  (bind _speed (Variables|Default|GetSpeed))
  (bind _returnvalue_2 (* DeltaSeconds _speed))
  (bind _returnvalue_3 (* _returnvalue _returnvalue_2))
  (Utilities|IsValid (Variables|Default|GetHead)
    (:Is%20Valid
      (Transformation|AddActorWorldOffset (Math|Vector|MakeVector (.x _returnvalue_3) (.y _returnvalue_3) 0.0) true))
    (:Is%20Not%20Valid
      (bind _returnvalue_4 (Actor|GetActorOfClass "/Game/FrazierContent/Entity/Head/BP_HeadCharacter.BP_HeadCharacter_C"))
      (Variables|Default|SetHead _returnvalue_4))))

(event EventBeginPlay
  (Utilities|Time|SetTimerbyEvent (delegate Custom|Destroy) (Variables|Default|GetTimeTillAutoDestroy)))

(event Collision|EventHit
  (params (MyComp :type Primitive%20Component%20Object%20Reference) (Other :type Actor%20Object%20Reference) (OtherComp :type Primitive%20Component%20Object%20Reference) (bSelfMoved :type Boolean) (HitLocation :type Vector :default "0, 0, 0") (HitNormal :type Vector :default "0, 0, 0") (NormalImpulse :type Vector :default "0, 0, 0") (Hit :type Hit%20Result%20Structure%20%28by%20ref%29))
  (bind _asbp_head_character (Utilities|Casting|CastToBP_HeadCharacter Other)
    (:then
      (CallFunction|DealDamage _asbp_head_character))
    (:CastFailed
      _))
  (CallFunction|Destroy))

(fn ConstructionScript)