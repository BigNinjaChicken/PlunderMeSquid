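; BP_ArmoredEnemy is an armored enemy variant that extends a parent Blueprint's spawn and damage behavior.
; On BeginPlay it runs the parent logic, then sets Health to 20.
; Each TakeDamage call shrinks the Mesh to 90% of its current world scale before passing to the parent handler, so the shrink compounds with every hit.
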(event EventBeginPlay
  (|CallParentFunction)
  (Variables|Default|SetHealth 2e+01))

(event EventTakeDamage
  (Transformation|SetWorldScale3D (Variables|Character|GetMesh) (* (Transformation|GetWorldScale (Variables|Character|GetMesh)) 0.9))
  (|CallParentFunction))

(fn ConstructionScript
  (|CallParentFunction))