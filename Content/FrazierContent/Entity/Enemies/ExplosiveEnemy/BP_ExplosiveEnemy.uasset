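; BP_ExplosiveEnemy is an enemy that explodes when it dies.
; On Death it draws a debug sphere, runs a sphere overlap at its location using ExplosiveRadius, then calls the parent death logic.
; Overlapped actors are cast to BP_Entity to choose the DealDamage amount, which is higher for the head character than for other entities.
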(event EventDeath
  (Rendering|Debug|DrawDebugSphere (Transformation|GetActorLocation) (Variables|Default|GetExplosiveRadius) 12 "(R=1.000000,G=0.457165,B=0.147349,A=1.000000)" 0.0)
  (bind _outactors (Collision|SphereOverlapActors (Transformation|GetActorLocation) (Variables|Default|GetExplosiveRadius) (Variables|Default|GetObject%20Types) 0))
  (for _array_element _outactors
    (bind _asbp_entity (Utilities|Casting|CastToBP_Entity _array_element))
    (if (!= _asbp_entity "/Game/FrazierContent/Entity/Head/BP_HeadCharacter.BP_HeadCharacter")
      (CallFunction|DealDamage 0 1e+01)
      (else
        (CallFunction|DealDamage 0 3e+01))))
  (|CallParentFunction))

(fn ConstructionScript
  (|CallParentFunction))