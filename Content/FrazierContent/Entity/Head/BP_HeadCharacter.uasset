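; Head character Blueprint that tracks health, owns the health HUD and starts ocean ambience and background music on BeginPlay.
; Tick feeds the health ratio into the liquid health widget's dynamic material.
; TakeDamge plays an attached damage sound and scales music pitch with remaining health, without changing Health itself.
; Death quits the game, and UpdatePlayerList caches all BP_RootCharacter actors.
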(event Custom|UpdatePlayerList
  (bind _outactors (Actor|GetAllActorsOfClass "/Game/FrazierContent/Entity/Player/BP_RootCharacter.BP_RootCharacter_C"))
  (Variables|Default|SetAllPlayers _outactors))

(event Custom|TakeDamge
  (Audio|Components|Audio|SetPitchMultiplier (Variables|Default|GetMusic) (Utilities|ScaleRange (Variables|Default|GetHealth) (Variables|Default|GetMaxHealth) 0.0 1.0 2.0))
  (Audio|SpawnSoundAttached "/Game/FrazierContent/Sounds/SW_Damage.SW_Damage" (Variables|Character|GetMesh) "None" "0, 0, 0" "0, 0, 0" "KeepRelativeOffset" false 1.0 1.0 0.0 0 0))

(event EventBeginPlay
  (Utilities|FlowControl|Sequence
    (:then_0
      (Variables|Default|SetHealth (Variables|Default|GetMaxHealth)))
    (:then_1
      (bind _returnvalue (UserInterface|CreateWidget "/Game/ArtinContent/BasicPresets/LiquidHealth/WD_LiquidHealth.WD_LiquidHealth_C"))
      (bind _output_get (Variables|Default|SetHud _returnvalue))
      (UserInterface|Viewport|AddtoViewport _output_get 0))
    (:then_2
      (Audio|PlaySound2D "/Game/FrazierContent/Sounds/SW_oceanwaves.SW_oceanwaves" 0.3 1.0 0.0 0 0)
      (bind _returnvalue_2 (Audio|SpawnSound2D "/Game/FrazierContent/Sounds/SW_relaxingbackgroundmusic.SW_relaxingbackgroundmusic" 1.0 1.0 0.0 0))
      (Variables|Default|SetMusic _returnvalue_2))))

(event EventTick
  (params (DeltaSeconds :type Float%20%28single-precision%29))
  (|CallParentFunction DeltaSeconds)
  (Utilities|FlowControl|Sequence
    (:then_0
      (bind _returnvalue (Appearance|GetDynamicMaterial (Variables|/Game/ArtinContent/BasicPresets/LiquidHealth/WD_LiquidHealth.WD_LiquidHealth_C|GetLiquitHealth (Variables|Default|GetHud)) :!class /Script/UMG.Image))
      (Rendering|Material|SetScalarParameterValue _returnvalue "Percentage" (/ (Variables|Default|GetHealth) (Variables|Default|GetMaxHealth)) :!class /Script/Engine.MaterialInstanceDynamic))))

(event EventDeath
  (Game|QuitGame 0 "Quit" false))

(fn ConstructionScript)