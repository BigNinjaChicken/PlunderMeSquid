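; Player pawn for local three-player tentacle play, where one controller's input drives three tentacles.
; On BeginPlay it detaches its camera boom, starts mesh bobbing, adds arrow-key, WASD and gamepad mapping contexts, and spawns two BP_TentacleMechanics pawns with default controllers.
; Per-player Enhanced Input move and grab actions drive itself as player one and are forwarded to the spawned pawns.
; It also handles quitting and overrides TakeDamage to do nothing.
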(event Input|EnhancedActionEvents|EnhancedInputActionIA_Grab_Player1
  (params (ActionValue :type Boolean) (ElapsedSeconds :type Float%20%28double-precision%29) (TriggeredSeconds :type Float%20%28double-precision%29) (InputAction :type Input%20Action%20Object%20Reference :default "/Game/FrazierContent/Input/FirstPlayer/IA_Grab_Player1.IA_Grab_Player1"))
  (:Triggered
    (Default|PlayerInputGrab self)))

(event Input|EnhancedActionEvents|EnhancedInputActionIA_Move_Player2
  (params (ActionValue :type Vector%202D%20Structure) (ElapsedSeconds :type Float%20%28double-precision%29) (TriggeredSeconds :type Float%20%28double-precision%29) (InputAction :type Input%20Action%20Object%20Reference :default "/Game/FrazierContent/Input/FirstPlayer/IA_Move_Player2.IA_Move_Player2"))
  (:Triggered
    (Default|PlayerInputMove (Variables|Default|GetPlayer2) (.x ActionValue) (.y ActionValue))))

(event Input|EnhancedActionEvents|EnhancedInputActionIA_Move_Player1
  (params (ActionValue :type Vector%202D%20Structure) (ElapsedSeconds :type Float%20%28double-precision%29) (TriggeredSeconds :type Float%20%28double-precision%29) (InputAction :type Input%20Action%20Object%20Reference :default "/Game/FrazierContent/Input/FirstPlayer/IA_Move_Player1.IA_Move_Player1"))
  (:Triggered
    (Default|PlayerInputMove self (.x ActionValue) (.y ActionValue))))

(event Input|EnhancedActionEvents|EnhancedInputActionIA_Grab_Player2
  (params (ActionValue :type Boolean) (ElapsedSeconds :type Float%20%28double-precision%29) (TriggeredSeconds :type Float%20%28double-precision%29) (InputAction :type Input%20Action%20Object%20Reference :default "/Game/FrazierContent/Input/FirstPlayer/IA_Grab_Player2.IA_Grab_Player2"))
  (:Triggered
    (Default|PlayerInputGrab (Variables|Default|GetPlayer2))))

(event Input|EnhancedActionEvents|EnhancedInputActionIA_Quit
  (params (ActionValue :type Boolean) (ElapsedSeconds :type Float%20%28double-precision%29) (TriggeredSeconds :type Float%20%28double-precision%29) (InputAction :type Input%20Action%20Object%20Reference :default "/Game/FrazierContent/Input/FirstPlayer/IA_Quit.IA_Quit"))
  (:Triggered
    (Game|QuitGame 0 "Quit" false)))

(event Input|EnhancedActionEvents|EnhancedInputActionIA_Move_Player3
  (params (ActionValue :type Vector%202D%20Structure) (ElapsedSeconds :type Float%20%28double-precision%29) (TriggeredSeconds :type Float%20%28double-precision%29) (InputAction :type Input%20Action%20Object%20Reference :default "/Game/FrazierContent/Input/FirstPlayer/IA_Move_Player3.IA_Move_Player3"))
  (:Triggered
    (Default|PlayerInputMove (Variables|Default|GetPlayer3) (.x ActionValue) (.y ActionValue))))

(event Input|EnhancedActionEvents|EnhancedInputActionIA_Grab_Player3
  (params (ActionValue :type Boolean) (ElapsedSeconds :type Float%20%28double-precision%29) (TriggeredSeconds :type Float%20%28double-precision%29) (InputAction :type Input%20Action%20Object%20Reference :default "/Game/FrazierContent/Input/FirstPlayer/IA_Grab_Player3.IA_Grab_Player3"))
  (:Triggered
    (Default|PlayerInputGrab (Variables|Default|GetPlayer3))))

(event EventBeginPlay
  (bind _index_0 (Variables|Default|GetIndex_0))
  (bind _returnvalue (Game|GetPlayerController _index_0))
  (bind _returnvalue_2 (PlayerController|LocalPlayerSubsystems|GetEnhancedInputLocalPlayerSubsystem _returnvalue))
  (Utilities|FlowControl|Sequence
    (:then_0
      (Transformation|DetachFromComponent (Variables|Camera|GetCameraBoom_0) "KeepWorld" "KeepWorld" "KeepWorld" true))
    (:then_1
      (CallFunction|MeshBobb))
    (:then_2
      (Utilities|IsValid _returnvalue_2
        (:Is%20Valid
          (Input|AddMappingContext _returnvalue_2 "/Game/FrazierContent/Input/IMC_ArrowKeysAndGamePad.IMC_ArrowKeysAndGamePad" 0 "(bIgnoreAllPressedKeysUntilRelease=True,bForceImmediately=False)")
          (Input|AddMappingContext _returnvalue_2 "/Game/FrazierContent/Input/IMC_GamePad.IMC_GamePad" 0 "(bIgnoreAllPressedKeysUntilRelease=True,bForceImmediately=False)")
          (Input|AddMappingContext _returnvalue_2 "/Game/FrazierContent/Input/IMC_WASD.IMC_WASD" 0 "(bIgnoreAllPressedKeysUntilRelease=True,bForceImmediately=False)"))))
    (:then_3
      (bind _returnvalue_3 (Game|SpawnActorfromClass "/Game/FrazierContent/Entity/Player/BP_TentacleMechanics.BP_TentacleMechanics_C" (Transformation|GetActorTransform) "Undefined" 0 0 0))
      (bind _output_get (Variables|Default|SetPlayer2 _returnvalue_3))
      (Pawn|SpawnDefaultController _output_get)
      (bind _returnvalue_4 (Game|SpawnActorfromClass "/Game/FrazierContent/Entity/Player/BP_TentacleMechanics.BP_TentacleMechanics_C" (Transformation|GetActorTransform) "Undefined" 0 0 0))
      (bind _output_get_2 (Variables|Default|SetPlayer3 _returnvalue_4))
      (Pawn|SpawnDefaultController _output_get_2))))

(event EventTakeDamage)

(fn ConstructionScript)