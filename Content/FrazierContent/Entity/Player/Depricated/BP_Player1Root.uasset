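; Player 1 root character for local two-player play, kept in a deprecated folder, that receives both players' input and offers a quit action.
; On BeginPlay, Setup spawns Player 2 at an offset, has a new PlayerController possess it, then spawns a head character with a default controller and updates its player list.
; Player 1 move and grab inputs act on this character, while Player 2's are forwarded directly to the spawned pawn.
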(event Input|EnhancedActionEvents|EnhancedInputActionIA_Grab_Player1
  (params (ActionValue :type Boolean) (ElapsedSeconds :type Float%20%28double-precision%29) (TriggeredSeconds :type Float%20%28double-precision%29) (InputAction :type Input%20Action%20Object%20Reference :default "/Game/FrazierContent/Input/FirstPlayer/IA_Grab_Player1.IA_Grab_Player1"))
  (:Triggered
    (Default|PlayerInputGrab self)))

(event Input|EnhancedActionEvents|EnhancedInputActionIA_Move_Player2
  (params (ActionValue :type Vector%202D%20Structure) (ElapsedSeconds :type Float%20%28double-precision%29) (TriggeredSeconds :type Float%20%28double-precision%29) (InputAction :type Input%20Action%20Object%20Reference :default "/Game/FrazierContent/Input/FirstPlayer/IA_Move_Player2.IA_Move_Player2"))
  (:Triggered
    (Default|PlayerInputMove (Variables|Kraken|GetPlayer2) (.x ActionValue) (.y ActionValue))))

(event Input|EnhancedActionEvents|EnhancedInputActionIA_Move_Player1
  (params (ActionValue :type Vector%202D%20Structure) (ElapsedSeconds :type Float%20%28double-precision%29) (TriggeredSeconds :type Float%20%28double-precision%29) (InputAction :type Input%20Action%20Object%20Reference :default "/Game/FrazierContent/Input/FirstPlayer/IA_Move_Player1.IA_Move_Player1"))
  (:Triggered
    (Default|PlayerInputMove self (.x ActionValue) (.y ActionValue))))

(event Input|EnhancedActionEvents|EnhancedInputActionIA_Grab_Player2
  (params (ActionValue :type Boolean) (ElapsedSeconds :type Float%20%28double-precision%29) (TriggeredSeconds :type Float%20%28double-precision%29) (InputAction :type Input%20Action%20Object%20Reference :default "/Game/FrazierContent/Input/FirstPlayer/IA_Grab_Player2.IA_Grab_Player2"))
  (:Triggered
    (Default|PlayerInputGrab (Variables|Kraken|GetPlayer2))))

(event Input|EnhancedActionEvents|EnhancedInputActionIA_Quit
  (params (ActionValue :type Boolean) (ElapsedSeconds :type Float%20%28double-precision%29) (TriggeredSeconds :type Float%20%28double-precision%29) (InputAction :type Input%20Action%20Object%20Reference :default "/Game/FrazierContent/Input/FirstPlayer/IA_Quit.IA_Quit"))
  (:Triggered
    (Game|QuitGame 0 "Quit" false)))

(event EventBeginPlay
  (CallFunction|Setup)
  (|CallParentFunction))

(fn ConstructionScript
  (|CallParentFunction))

(fn Setup
  (bind _capsulecomponent (Variables|Default|GetCapsuleComponent))
  (bind _offset (Variables|Setup|GetOffset))
  (bind _returnvalue (Transformation|GetWorldTransform _capsulecomponent))
  (bind _returnvalue_2 (+ _offset (.y (.location _returnvalue))))
  (bind _returnvalue_3 (+ _offset (.x (.location _returnvalue))))
  (bind _returnvalue_4 (Math|Transform|MakeTransform (Math|Vector|MakeVector _returnvalue_3 _returnvalue_2 (.z (.location _returnvalue))) (.rotation _returnvalue) (.scale _returnvalue)))
  (bind _returnvalue_5 (Game|SpawnActorfromClass "/Game/FrazierContent/Entity/Player/Depricated/BP_Player2Root.BP_Player2Root_C" _returnvalue_4 "Undefined" 0 0))
  (bind _output_get (Variables|Kraken|SetPlayer2 _returnvalue_5))
  (bind _returnvalue_6 (Game|SpawnActorfromClass "/Script/Engine.PlayerController" (Transformation|GetActorTransform _output_get) "Undefined" 0 0))
  (Pawn|Possess _returnvalue_6 _output_get)
  (bind _returnvalue_7 (Game|SpawnActorfromClass "/Game/FrazierContent/Entity/Head/BP_HeadCharacter.BP_HeadCharacter_C" _returnvalue_4 "Undefined" 0 0))
  (Pawn|SpawnDefaultController _returnvalue_7)
  (Default|UpdatePlayerList _returnvalue_7))