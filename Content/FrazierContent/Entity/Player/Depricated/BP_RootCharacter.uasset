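; Player character tethered to a shared BP_HeadCharacter, able to grab and throw enemies and barrels or activate interactables.
; Tick pulls it back toward the Head beyond a radius and centers the camera boom there, scaling its offset by the farthest player's distance.
; A timeline-driven gate enforces grab cooldowns; sphere overlaps find targets, which attach to a tentacle socket.
; Throws auto-aim at an enemy ahead and move by swept offsets.
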(event Custom|MeshBobb
  (Components|Timeline|SetPlayRate (Variables|Default|GetT_Bobb) 0.4)
  (bind _value (Timeline|T_Bobb PlayFromStart)
    (:Update
      (Transformation|SetRelativeLocation (Variables|Character|GetMesh) (Math|Vector|MakeVector 0.0 0.0 (Math|Float|Lerp -9e+01 -6e+01 _value)) false false))
    (:Finished
      (Timeline|T_Bobb PlayFromStart))))

(event Custom|PlayerInput%20Move
  (params (X :type Float%20%28double-precision%29) (Y :type Float%20%28double-precision%29))
  (bind _followcamera (Variables|Camera|GetFollowCamera))
  (bind _returnvalue (Transformation|GetWorldRotation _followcamera))
  (Pawn|Input|AddMovementInput (Math|Vector|GetRightVector (Math|Rotator|MakeRotator (.roll _returnvalue) 0.0 (.yaw _returnvalue))) X false)
  (Pawn|Input|AddMovementInput (Math|Vector|GetForwardVector (Math|Rotator|MakeRotator 0.0 0.0 (.yaw (Transformation|GetWorldRotation _followcamera)))) Y false))

(event Custom|AddBackCollsion
  (Collision|SetCollisionResponsetoChannel (Variables|Default|GetCapsuleComponent) "ECC_GameTraceChannel1" "ECR_Block"))

(event Custom|PlayerInput%20Grab
  (bind _returnvalue (Transformation|GetActorLocation))
  (bind _returnvalue_2 (Transformation|GetActorForwardVector))
  (bind _grabhitboxdistance (Variables|Grab|GetGrabHitBoxDistance))
  (bind _returnvalue_3 (* _returnvalue_2 _grabhitboxdistance))
  (bind _returnvalue_4 (+ _returnvalue _returnvalue_3))
  (Utilities|FlowControl|Gate false
    (:Exit
      (Utilities|IsValid (Variables|Grab|GetPickedUpEnemy)
        (:Is%20Valid
          (Variables|Grab|SetThrowableActor (Variables|Grab|GetPickedUpEnemy))
          (CallFunction|GrabCooldown 2.0 :!label _label)
          (Utilities|IsValid (Variables|Grab|GetThrowableActor)
            (:Is%20Valid
              (Variables|/Game/FrazierContent/Entity/BP_PickupableEntity.BP_PickupableEntity_C|SetCanTakeHitDamage (Variables|Grab|GetThrowableActor) true)
              (Transformation|DetachFromActor (Variables|Grab|GetThrowableActor) "KeepWorld" "KeepWorld" "KeepWorld")
              (Components|Timeline|SetPlayRate (Variables|Default|GetT_Throw) (/ 1.0 (Variables|Grab|GetEnemyThrowDuration)))
              (Grab|GetEnemiesInfront)
              (Timeline|T_Throw PlayFromStart
                (:Update
                  (Utilities|IsValid (Variables|Grab|GetThrowableActor)
                    (:Is%20Valid
                      (Transformation|AddActorWorldOffset (Variables|Grab|GetThrowableActor) (* (Variables|Grab|GetForwardVector) (Variables|Grab|GetThrowSpeed) (Utilities|Time|GetWorldDeltaSeconds)) true))))
                (:Finished
                  (Utilities|IsValid (Variables|Grab|GetThrowableActor)
                    (:Is%20Valid
                      (Variables|/Game/FrazierContent/Entity/BP_PickupableEntity.BP_PickupableEntity_C|SetCanTakeHitDamage (Variables|Grab|GetThrowableActor) false)
                      (Utilities|IsValid (Variables|Grab|GetPickedUpEnemy)
                        (:Is%20Valid
                          (Variables|/Game/FrazierContent/Entity/Enemies/RootEnemy/BP_RootEnemy.BP_RootEnemy_C|SetReady (Variables|Grab|GetPickedUpEnemy) true))
                        (:Is%20Not%20Valid
                          _))
                      (Utilities|Time|SetTimerbyEvent (delegate Custom|AddBackCollsion) 0.1)
                      (Variables|Grab|SetPickedUpEnemy 0)
                      (Variables|Grab|SetPickedUpBarrel 0))))))
            (:Is%20Not%20Valid
              (CallFunction|AddBackCollsion))))
        (:Is%20Not%20Valid
          (Utilities|IsValid (Variables|Grab|GetPickedUpBarrel)
            (:Is%20Valid
              (Variables|Grab|SetThrowableActor (Variables|Grab|GetPickedUpBarrel))
              (goto _label))
            (:Is%20Not%20Valid
              (CallFunction|GrabCooldown 2.0)
              (bind _outactors (Collision|SphereOverlapActors _returnvalue_4 (Variables|Grab|GetSphereRadius) (Variables|Grab|GetObject%20Types) 0))
              (Rendering|Debug|DrawDebugSphere _returnvalue_4 0.0 12 "(R=1.000000,G=0.000000,B=0.073746,A=1.000000)" 0.1 2.0)
              (bind _array_element (Utilities|Array|ForEachLoopwithBreak _outactors :!label _label_2)
                (:LoopBody
                  (bind _asbp_root_enemy (Utilities|Casting|CastToBP_RootEnemy _array_element)
                    (:then
                      (if (Variables|/Game/FrazierContent/Entity/Enemies/RootEnemy/BP_RootEnemy.BP_RootEnemy_C|GetIsPickupable _asbp_root_enemy)
                        (Variables|Grab|SetPickedUpEnemy _asbp_root_enemy)
                        (CallFunction|PickUp :!label _label_3)
                        (goto _label_2 Break)))
                    (:CastFailed
                      (bind _asbp_barrel (Utilities|Casting|CastToBP_Barrel _array_element)
                        (:then
                          (Variables|Grab|SetPickedUpBarrel _asbp_barrel)
                          (goto _label_3))
                        (:CastFailed
                          (bind _asbp_interactable (Utilities|Casting|CastToBP_Interactable _array_element))
                          (Default|Activate _asbp_interactable)
                          (goto _label_2 Break))))))))))))))

(event Custom|PickUp
  (bind _pickedupenemy (Variables|Grab|GetPickedUpEnemy))
  (Utilities|IsValid (Variables|Grab|GetPickedUpEnemy)
    (:Is%20Valid
      (Variables|/Game/FrazierContent/Entity/Enemies/RootEnemy/BP_RootEnemy.BP_RootEnemy_C|SetReady _pickedupenemy false)
      (AI|Navigation|StopMovement (AI|GetAIController _pickedupenemy))
      (Grab|AttachtoTentacle _pickedupenemy))
    (:Is%20Not%20Valid
      (Utilities|IsValid (Variables|Grab|GetPickedUpBarrel)
        (:Is%20Valid
          (Grab|AttachtoTentacle (Variables|Grab|GetPickedUpBarrel))))))
  (CallFunction|GrabCooldown 1.0)
  (Collision|SetCollisionResponsetoChannel (Variables|Default|GetCapsuleComponent) "ECC_GameTraceChannel1" "ECR_Overlap"))

(event Custom|GrabCooldown
  (params (Duration :type Float%20%28double-precision%29))
  (bind _returnvalue (Transformation|GetActorLocation))
  (bind _returnvalue_2 (Transformation|GetActorForwardVector))
  (bind _grabhitboxdistance (Variables|Grab|GetGrabHitBoxDistance))
  (bind _returnvalue_3 (* _returnvalue_2 _grabhitboxdistance))
  (bind _returnvalue_4 (+ _returnvalue _returnvalue_3))
  (Components|Timeline|SetPlayRate (Variables|Default|GetT_Cooldown) (/ 1.0 Duration))
  (Timeline|T_Cooldown PlayFromStart
    (:Update
      (Utilities|FlowControl|Gate false) ; enters at Close
    )
    (:Finished
      (Utilities|FlowControl|Gate false) ; enters at Open
    )))

(event EventBeginPlay
  (Utilities|FlowControl|Sequence
    (:then_0
      (Transformation|DetachFromComponent (Variables|Camera|GetCameraBoom) "KeepWorld" "KeepWorld" "KeepWorld" true))
    (:then_1
      (CallFunction|MeshBobb))
    (:then_2
      (Game|SpawnActorfromClass "/Game/FrazierContent/Entity/Player/PC_Tentacle.PC_Tentacle_C" (Transformation|GetActorTransform) "Undefined" 0 0))
    (:then_3
      (bind _asplayer_controller (Utilities|Casting|CastToPlayerController (Pawn|GetController)))
      (Utilities|IsValid (PlayerController|LocalPlayerSubsystems|GetEnhancedInputLocalPlayerSubsystem _asplayer_controller)
        (:Is%20Valid
          (Input|AddMappingContext (PlayerController|LocalPlayerSubsystems|GetEnhancedInputLocalPlayerSubsystem _asplayer_controller) "/Game/FrazierContent/Input/IMC_ArrowKeysAndGamePad.IMC_ArrowKeysAndGamePad" 0 "(bIgnoreAllPressedKeysUntilRelease=True,bForceImmediately=False)"))))))

(event EventTick
  (params (DeltaSeconds :type Float%20%28single-precision%29))
  (Utilities|FlowControl|Sequence
    (:then_0
      (if (not (Utilities|IsValid (Variables|Default|GetHead)))
        (bind _returnvalue (Actor|GetActorOfClass "/Game/FrazierContent/Entity/Head/BP_HeadCharacter.BP_HeadCharacter_C"))
        (Variables|Default|SetHead _returnvalue)
        (else
          (Utilities|FlowControl|Sequence
            (:then_0
              (if (> (Math|Vector|Distance(Vector) (Transformation|GetActorLocation (Variables|Default|GetHead)) (Transformation|GetActorLocation)) (Variables|Tether|GetMaxRadius))
                (CallFunction|PlayerInputMove (.x (* (Math|Vector|Normalize (Math|Vector|GetUnitDirection(Vector) (Transformation|GetActorLocation) (Transformation|GetActorLocation (Variables|Default|GetHead)))) (Variables|Tether|GetStrength))) (.z (* (Math|Vector|Normalize (Math|Vector|GetUnitDirection(Vector) (Transformation|GetActorLocation) (Transformation|GetActorLocation (Variables|Default|GetHead)))) (Variables|Tether|GetStrength))))))))))
    (:then_2
      (Utilities|IsValid (Variables|Default|GetHead)
        (:Is%20Valid
          (Transformation|SetWorldRotation (Variables|Camera|GetFollowCamera) (Math|Rotator|FindLookatRotation (Transformation|GetWorldLocation (Variables|Camera|GetFollowCamera)) (Transformation|GetWorldLocation (Variables|/Script/Engine.Character|GetCapsuleComponent (Variables|Default|GetHead)))) false false)
          (Transformation|SetWorldLocation (Variables|Camera|GetCameraBoom) (Transformation|GetWorldLocation (Variables|/Script/Engine.Character|GetCapsuleComponent (Variables|Default|GetHead))) false false)
          (bind _greatestdistance (Camera|GetFarthestTentacle))
          (Variables|/Script/Engine.SpringArmComponent|SetTargetOffset (Variables|Camera|GetCameraBoom) (Math|Vector|Lerp(Vector) (Variables|Camera|GetMinCamDistance) (Variables|Camera|GetMaxCamDistance) (Math|Float|Clamp(Float) (/ (- _greatestdistance (Variables|Camera|GetMinCamOffset)) (Variables|Camera|GetMaxCamOffset)) 0.4))))))))

(event EventTakeDamage)

(fn ConstructionScript)

(fn GetFarthestTentacle
  (for _array_element (Variables|/Game/FrazierContent/Entity/Head/BP_HeadCharacter.BP_HeadCharacter_C|GetAllPlayers (Variables|Default|GetHead))
    (if (> (Transformation|GetDistanceTo _array_element (Variables|Default|GetHead)) (LocalVariables|GetFarthest))
      (bind _output_get (LocalVariables|SetFarthest (Transformation|GetDistanceTo _array_element (Variables|Default|GetHead))))))
  (return _output_get))

(fn AttachtoTentacle
  (params (Actor :type BP%20Pickupable%20Entity%20Object%20Reference))
  (Transformation|AttachActorToActor Actor self "Bone_006" "SnapToTarget" "KeepWorld" "KeepWorld" true)
  (Transformation|SetActorLocation Actor (+ (* (Transformation|GetActorForwardVector) (Variables|Grab|GetGrabHitBoxDistance)) (Transformation|GetActorLocation)) false false))

(fn GetEnemiesInfront
  (bind _self self)
  (bind _outhits (Collision|MultiSphereTraceForObjects (Utilities|ApplyForwardtoLocation _self 1.5e+02) (Utilities|ApplyForwardtoLocation _self 5.5e+02) (LocalVariables|GetRadius) (LocalVariables|GetObjectsToCast) false 0 "None"))
  (bind _array_element (Utilities|Array|ForEachLoopwithBreak _outhits)
    (:LoopBody
      (bind _asbp_root_enemy (Utilities|Casting|CastToBP_RootEnemy (.HitActor (Collision|BreakHitResult _array_element))))
      (Variables|Grab|SetForwardVector (Math|Vector|GetUnitDirection(Vector) (Transformation|GetActorLocation) (Transformation|GetActorLocation _asbp_root_enemy)))
      (return))
    (:Completed
      (Variables|Grab|SetForwardVector (Transformation|GetActorForwardVector))
      (return))))