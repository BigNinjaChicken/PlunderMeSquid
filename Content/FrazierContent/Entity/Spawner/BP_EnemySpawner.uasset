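; BP_EnemySpawner spawns an enemy of a set class at its own location when no enemy is nearby.
; On BeginPlay or CheckSpawnEnemy, it runs a sphere overlap and looks for any BP_RootEnemy.
; If none is found, a timeline scaled to the Timer duration delays the spawn, then a default controller is spawned for the new actor's Instigator.
; The construction script sizes BoundingSphere to the search radius.
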(event Custom|CheckSpawnEnemy
  (bind _outactors (Collision|SphereOverlapActors (Transformation|GetActorLocation) (Variables|Default|GetSphere%20Radius) (Variables|Default|GetObject%20Types) 0))
  (bind _return (CallFunction|IsThereEnemy _outactors))
  (if (not _return)
    (Components|Timeline|SetPlayRate (Variables|Default|GetSpawnEnemyTimer) (/ 1.0 (Variables|Default|GetTimer)))
    (Timeline|SpawnEnemyTimer PlayFromStart
      (:Finished
        (bind _returnvalue (Game|SpawnActorfromClass (Variables|Default|GetSpawnedEnemy) (Transformation|GetActorTransform) "Undefined" 0 0))
        (Pawn|SpawnDefaultController (Variables|/Script/Engine.Actor|GetInstigator _returnvalue))))))

(event EventBeginPlay
  (bind _outactors (Collision|SphereOverlapActors (Transformation|GetActorLocation) (Variables|Default|GetSphere%20Radius) (Variables|Default|GetObject%20Types) 0))
  (bind _return (CallFunction|IsThereEnemy _outactors))
  (if (not _return)
    (Components|Timeline|SetPlayRate (Variables|Default|GetSpawnEnemyTimer) (/ 1.0 (Variables|Default|GetTimer)))
    (Timeline|SpawnEnemyTimer PlayFromStart
      (:Finished
        (bind _returnvalue (Game|SpawnActorfromClass (Variables|Default|GetSpawnedEnemy) (Transformation|GetActorTransform) "Undefined" 0 0))
        (Pawn|SpawnDefaultController (Variables|/Script/Engine.Actor|GetInstigator _returnvalue))))))

(fn ConstructionScript
  (Components|Sphere|SetSphereRadius (Variables|Default|GetBoundingSphere) (Variables|Default|GetSphere%20Radius) true))

(fn IsThereEnemy
  (params (Array :type Array%20of%20Actor%20Object%20References))
  (for _array_element Array
    (Utilities|Casting|CastToBP_RootEnemy _array_element)
    (return true))
  (return false))