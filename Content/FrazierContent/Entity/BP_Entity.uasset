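; BP_Entity is a base character Blueprint that provides health, damage, death and a temporary speed boost.
; DealDamage subtracts from a target's Health and calls its TakeDamage event, which is left empty for child classes to implement.
; Tick polls Health and calls Death at zero or below, destroying the actor.
; SpeedFruitEffect multiplies walk speed, using a timeline with play rate scaled by duration to restore it when finished.
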(event Custom|Death
  (Actor|DestroyActor))

(event Custom|SpeedFruitEffect
  (params (Duration :type Float%20%28double-precision%29))
  (Components|Timeline|SetPlayRate (Variables|Default|GetSpeedTimer) (/ 1.0 Duration))
  (bind _output_get (Variables|Default|SetDefault%20Speed (Variables|/Script/Engine.CharacterMovementComponent|GetMaxWalkSpeed (Variables|Character|GetCharacterMovement))))
  (Variables|/Script/Engine.CharacterMovementComponent|SetMaxWalkSpeed (Variables|Character|GetCharacterMovement) (* _output_get (Variables|Default|GetSpeedMultiplier)))
  (Timeline|SpeedTimer PlayFromStart
    (:Finished
      (Variables|/Script/Engine.CharacterMovementComponent|SetMaxWalkSpeed (Variables|Character|GetCharacterMovement) (Variables|Default|GetDefault%20Speed)))))

(event Custom|DealDamage
  (params (Target :type BP%20Entity%20Object%20Reference) (Damage :type Float%20%28double-precision%29))
  (Variables|BP_Entity_C|SetHealth Target (- (Variables|BP_Entity_C|GetHealth Target) Damage))
  (CallFunction|TakeDamage Target))

(event Custom|TakeDamage)

(event EventTick
  (params (DeltaSeconds :type Float%20%28single-precision%29))
  (if (<= (Variables|Default|GetHealth) 0.0)
    (CallFunction|Death)))

(fn ConstructionScript)