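; BP_RootEnemy is an enemy ship base that can fire cannons and breaks apart on collision, releasing crew.
; It tracks its own and the player head's locations, which ShootEvent uses to spawn a cannon actor toward the head, with a timeline cooldown re-enabling shooting.
; When hit damage is enabled, striking a solid hazard, root character or fellow enemy triggers death, killing both enemies in the latter case.
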(event Custom|ShootEvent
  (bind _selflocation (Variables|Default|GetSelfLocation))
  (bind _headlocation (Variables|Default|GetHeadLocation))
  (bind _selflocation_2 (Variables|Default|GetSelfLocation))
  (bind _returnvalue (Math|Rotator|FindLookatRotation _selflocation _headlocation))
  (bind _returnvalue_2 (Math|Vector|GetForwardVector _returnvalue))
  (bind _returnvalue_3 (* _returnvalue_2 5e+01))
  (bind _returnvalue_4 (+ _returnvalue_3 _selflocation_2))
  (Utilities|FlowControl|Sequence
    (:then_0
      (Components|Timeline|SetPlayRate (Variables|Default|GetCooldown) 0.25)
      (Timeline|Cooldown PlayFromStart
        (:Finished
          (Variables|Default|SetCanShoot true))))
    (:then_1
      (Game|SpawnActorfromClass "/Game/FrazierContent/Entity/Enemy/RootEnemy/BP_Canon.BP_Canon_C" (Math|Transform|MakeTransform (Math|Vector|MakeVector (.x _returnvalue_4) (.y _returnvalue_4) (+ (.z _returnvalue_4) 6e+01)) "0, 0, 0" "1.000000,1.000000,1.000000") "Undefined" 0 0))
    (:then_2
      (Audio|SpawnSoundatLocation "/Game/FrazierContent/Sounds/SW_CannonFire.SW_CannonFire" (Transformation|GetActorLocation) "0, 0, 0" 1.0 1.3 0.0 0 0))))

(event EventTick
  (params (DeltaSeconds :type Float%20%28single-precision%29))
  (Utilities|IsValid (Variables|Default|GetHead)
    (:Is%20Valid
      (Utilities|FlowControl|Sequence
        (:then_0
          (Variables|Default|SetSelfLocation (Transformation|GetActorLocation)))
        (:then_1
          (Variables|Default|SetHeadLocation (Transformation|GetActorLocation (Variables|Default|GetHead))))))
    (:Is%20Not%20Valid
      (bind _returnvalue (Actor|GetActorOfClass "/Game/FrazierContent/Entity/Head/BP_HeadCharacter.BP_HeadCharacter_C"))
      (Variables|Default|SetHead _returnvalue))))

(event EventBeginPlay
  (Utilities|FlowControl|Sequence
    (:then_0
      (Variables|Default|SetHealth 2e+01))
    (:then_1
      (Utilities|FlowControl|Delay 0.2)
      (Variables|Default|SetReady true))
    (:then_2
      (bind _returnvalue (Actor|GetActorOfClass "/Game/FrazierContent/Entity/Head/BP_HeadCharacter.BP_HeadCharacter_C"))
      (Variables|Default|SetHead _returnvalue))))

(event EventDeath
  (for _index (range 0 (- (Variables|Default|GetCrewAmount) 1))
    (Game|SpawnActorfromClass "/Game/FrazierContent/Entity/Enemy/Crew/BP_Crew.BP_Crew_C" (Transformation|GetActorTransform) "Undefined" 0 0))
  (Audio|SpawnSound2D "/Game/FrazierContent/Sounds/SW_Bell.SW_Bell" 1.0 1.0 0.0 0)
  (Audio|SpawnSoundAttached "/Game/FrazierContent/Sounds/SW_ShipBreak.SW_ShipBreak" (Variables|Character|GetMesh) "None" "0, 0, 0" "0, 0, 0" "KeepRelativeOffset" false 1.0 1.0 0.0 0 0)
  (Utilities|FlowControl|Delay 0.2)
  (Actor|DestroyActor))

(event Collision|EventHit
  (params (MyComp :type Primitive%20Component%20Object%20Reference) (Other :type Actor%20Object%20Reference) (OtherComp :type Primitive%20Component%20Object%20Reference) (bSelfMoved :type Boolean) (HitLocation :type Vector :default "0, 0, 0") (HitNormal :type Vector :default "0, 0, 0") (NormalImpulse :type Vector :default "0, 0, 0") (Hit :type Hit%20Result%20Structure%20%28by%20ref%29))
  (if (Variables|Default|GetCanTakeHitDamage)
    (Utilities|Casting|CastToBP_SoildHazard Other
      (:then
        _)
      (:CastFailed
        (Utilities|Casting|CastToBP_RootCharacter Other
          (:then
            _)
          (:CastFailed
            (bind _asbp_root_enemy (Utilities|Casting|CastToBP_RootEnemy Other))
            (Utilities|FlowControl|DoOnce false
              (:Completed
                (Default|Death _asbp_root_enemy)))))))
    (Utilities|FlowControl|DoOnce false
      (:Completed
        (CallFunction|Death)))))

(fn ConstructionScript)