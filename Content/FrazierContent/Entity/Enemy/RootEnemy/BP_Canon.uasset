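; BP_Canon is an enemy projectile that damages BP_HeadCharacter.
; On Tick it finds the head, captures the direction to it once, then sweeps straight along that heading in X and Y without homing.
; Overlapping the head applies Damage once and destroys it, while BP_RootCharacter only destroys it.
; A BeginPlay timer also destroys it, and the branch for damaging BP_RootEnemy is disconnected.
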(event Custom|Destroy
  (Actor|DestroyActor))

(event Custom|DealDamage
  (params (Target :type BP%20Entity%20Object%20Reference))
  (Utilities|FlowControl|DoOnce false
    (:Completed
      (Variables|/Game/FrazierContent/Entity/BP_Entity.BP_Entity_C|SetHealth Target (- (Variables|/Game/FrazierContent/Entity/BP_Entity.BP_Entity_C|GetHealth Target) (Variables|Default|GetDamage)))
      (bind _asbp_head_character (Utilities|Casting|CastToBP_HeadCharacter Target))
      (Default|TakeDamge _asbp_head_character))))

(event EventTick
  (params (DeltaSeconds :type Float%20%28single-precision%29))
  (Utilities|IsValid (Variables|Default|GetHead)
    (:Is%20Valid
      (Utilities|FlowControl|Sequence
        (:then_0
          (Utilities|FlowControl|DoOnce false
            (:Completed
              (Variables|Default|SetLocation (Math|Vector|Normalize (- (Transformation|GetActorLocation (Variables|Default|GetHead)) (Transformation|GetActorLocation))))
              (goto _label Open))))
        (:then_1
          (Utilities|FlowControl|Gate true :!label _label
            (:Exit
              (Transformation|AddActorWorldOffset (Math|Vector|MakeVector (.x (* (Variables|Default|GetLocation) (* DeltaSeconds (Variables|Default|GetSpeed)))) (.y (* (Variables|Default|GetLocation) (* DeltaSeconds (Variables|Default|GetSpeed)))) 0.0) true))))))
    (:Is%20Not%20Valid
      (bind _returnvalue (Actor|GetActorOfClass "/Game/FrazierContent/Entity/Head/BP_HeadCharacter.BP_HeadCharacter_C"))
      (Variables|Default|SetHead _returnvalue))))

(event Collision|EventActorBeginOverlap
  (params (OtherActor :type Actor%20Object%20Reference))
  (bind _asbp_head_character (Utilities|Casting|CastToBP_HeadCharacter OtherActor)
    (:then
      (CallFunction|DealDamage _asbp_head_character))
    (:CastFailed
      (Utilities|Casting|CastToBP_RootCharacter OtherActor)))
  (CallFunction|Destroy))

(event EventBeginPlay
  (Utilities|Time|SetTimerbyEvent (delegate Custom|Destroy) (Variables|Default|GetTimeTillAutoDestroy)))

(fn ConstructionScript)