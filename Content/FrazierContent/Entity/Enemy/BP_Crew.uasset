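; BP_Crew is an enemy-folder crew member that spawns screaming and gets flung in a random direction.
; On BeginPlay it attaches the scream sound, then a timeline scaled by flight time sweeps it forward while driving its height.
; Hitting a root or head character calls BlowUp, which, like hitting a hazard, just destroys the actor.
; A drown timer exists but is never triggered.
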(event Custom|BlowUp
  (Actor|DestroyActor))

(event EventBeginPlay
  (bind _returnvalue (Transformation|GetActorForwardVector))
  (bind _returnvalue_2 (Transformation|GetActorLocation))
  (bind _forwardspeed (Variables|Default|GetForwardSpeed))
  (Audio|SpawnSoundAttached "/Game/FrazierContent/Entity/Enemy/scream.scream" (Variables|Character|GetMesh) "None" "0, 0, 0" "0, 0, 0" "KeepRelativeOffset" true 0.1 1.0 0.0 "/Game/FrazierContent/Entity/Enemy/SA_Scream.SA_Scream" 0)
  (Transformation|SetActorRotation (Math|Rotator|MakeRotator 0.0 0.0 (* (Math|Random|RandomFloat) 3.6e+02)))
  (Components|Timeline|SetPlayRate (Variables|Default|GetT_Fly) (/ 1.0 (Variables|Default|GetTimeTakesToFly)))
  (bind _value (Timeline|T_Fly PlayFromStart)
    (:Update
      (Transformation|SetActorLocation (Math|Vector|MakeVector (+ (.x _returnvalue_2) (* (.x _returnvalue) _forwardspeed)) (+ (.y _returnvalue_2) (* (.y _returnvalue) _forwardspeed)) (Math|Float|Lerp 0.1 (Variables|Default|GetHeight) _value)) true false))))

(event Collision|EventHit
  (params (MyComp :type Primitive%20Component%20Object%20Reference) (Other :type Actor%20Object%20Reference) (OtherComp :type Primitive%20Component%20Object%20Reference) (bSelfMoved :type Boolean) (HitLocation :type Vector :default "0, 0, 0") (HitNormal :type Vector :default "0, 0, 0") (NormalImpulse :type Vector :default "0, 0, 0") (Hit :type Hit%20Result%20Structure%20%28by%20ref%29))
  (Utilities|Casting|CastToBP_RootCharacter Other
    (:then
      (CallFunction|BlowUp :!label _label))
    (:CastFailed
      (Utilities|Casting|CastToBP_HeadCharacter Other
        (:then
          (goto _label))
        (:CastFailed
          (Utilities|Casting|CastToBP_SoildHazard Other)
          (Actor|DestroyActor))))))

(fn ConstructionScript)