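; Tower enemy that fires a ring of four BP_Canon actors when its ShootEvent runs, with other behavior left to its parent class.
; The volley is based on the look-at rotation toward HeadLocation, with a shared random yaw offset and 90-degree spacing, spawning slightly out from and above the tower.
; A slowed timeline serves as the cooldown that re-enables CanShoot, while a pitched-up cannon sound plays.
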(event EventTick
  (params (DeltaSeconds :type Float%20%28single-precision%29))
  (|CallParentFunction DeltaSeconds))

(event EventShootEvent
  (bind _selflocation (Variables|Default|GetSelfLocation))
  (bind _headlocation (Variables|Default|GetHeadLocation))
  (bind _returnvalue (Math|Rotator|FindLookatRotation _selflocation _headlocation))
  (Utilities|FlowControl|Sequence
    (:then_0
      (Components|Timeline|SetPlayRate (Variables|Default|GetTimeline) 0.25)
      (Timeline|Timeline PlayFromStart
        (:Finished
          (Variables|Default|SetCanShoot true))))
    (:then_1
      (Variables|Default|SetRandomCannonRotation (Utilities|ScaleRange (Math|Random|RandomFloat) 0.0 1.0 -5e+01 5e+01))
      (for _index (range 0 3)
        (Variables|Default|SetCannonIndex _index)
        (Game|SpawnActorfromClass "/Game/FrazierContent/Entity/Enemy/RootEnemy/BP_Canon.BP_Canon_C" (Math|Transform|MakeTransform (Math|Vector|MakeVector (.x (+ (* (Math|Vector|GetForwardVector (Math|Rotator|MakeRotator (.roll _returnvalue) (.pitch _returnvalue) (+ (+ (.yaw _returnvalue) (Variables|Default|GetRandomCannonRotation)) (* (Variables|Default|GetCannonIndex) 9e+01)))) 5e+01) (Variables|Default|GetSelfLocation))) (.y (+ (* (Math|Vector|GetForwardVector (Math|Rotator|MakeRotator (.roll _returnvalue) (.pitch _returnvalue) (+ (+ (.yaw _returnvalue) (Variables|Default|GetRandomCannonRotation)) (* (Variables|Default|GetCannonIndex) 9e+01)))) 5e+01) (Variables|Default|GetSelfLocation))) (+ (.z (+ (* (Math|Vector|GetForwardVector (Math|Rotator|MakeRotator (.roll _returnvalue) (.pitch _returnvalue) (+ (+ (.yaw _returnvalue) (Variables|Default|GetRandomCannonRotation)) (* (Variables|Default|GetCannonIndex) 9e+01)))) 5e+01) (Variables|Default|GetSelfLocation))) 6e+01)) (Math|Rotator|MakeRotator (.roll _returnvalue) (.pitch _returnvalue) (+ (+ (.yaw _returnvalue) (Variables|Default|GetRandomCannonRotation)) (* (Variables|Default|GetCannonIndex) 9e+01))) "1.000000,1.000000,1.000000") "Undefined" 0 0)))
    (:then_2
      (Audio|SpawnSoundatLocation "/Game/FrazierContent/Sounds/SW_CannonFire.SW_CannonFire" (Transformation|GetActorLocation) "0, 0, 0" 1.0 1.3 0.0 0 0))))

(fn ConstructionScript
  (|CallParentFunction))