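; BP_Crew is an enemy crew actor that flies off screaming in a random direction when spawned.
; A timeline scaled by flight time sets its height while sweeping it forward, and Tick makes the attached scream louder as it nears the player head.
; Hitting the root or head character calls BlowUp, which, like hitting a solid hazard, simply destroys it.
; Drown timer logic exists but is never run.
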(event Custom|BlowUp
  (Actor|DestroyActor))

(event EventBeginPlay
  (bind _returnvalue (Transformation|GetActorForwardVector))
  (bind _returnvalue_2 (Transformation|GetActorLocation))
  (bind _forwardspeed (Variables|Default|GetForwardSpeed))
  (bind _returnvalue_3 (Audio|SpawnSoundAttached "/Game/FrazierContent/Sounds/SW_Scream.SW_Scream" (Variables|Character|GetMesh) "None" "0, 0, 0" "0, 0, 0" "KeepWorldPosition" true 1.0 1.0 0.0 0 0 false))
  (Variables|Default|SetScreamSound _returnvalue_3)
  (Transformation|SetActorRotation (Math|Rotator|MakeRotator 0.0 0.0 (* (Math|Random|RandomFloat) 3.6e+02)))
  (Components|Timeline|SetPlayRate (Variables|Default|GetT_Fly) (/ 1.0 (Variables|Default|GetTimeTakesToFly)))
  (bind _value (Timeline|T_Fly PlayFromStart)
    (:Update
      (Transformation|SetActorLocation (Math|Vector|MakeVector (+ (.x _returnvalue_2) (* (.x _returnvalue) _forwardspeed)) (+ (.y _returnvalue_2) (* (.y _returnvalue) _forwardspeed)) (Math|Float|Lerp 0.1 (Variables|Default|GetHeight) _value)) true false))))

(event EventTick
  (params (DeltaSeconds :type Float%20%28single-precision%29))
  (bind _screamsound (Variables|Default|GetScreamSound))
  (bind _maxscreamrange (Variables|Default|GetMaxScreamRange))
  (|CallParentFunction DeltaSeconds)
  (Utilities|IsValid (Variables|Default|GetPlayerHead)
    (:Is%20Valid
      (Utilities|IsValid _screamsound
        (:Is%20Valid
          (Audio|Components|Audio|SetVolumeMultiplier _screamsound (Utilities|ScaleRange (Math|Float|Min(Float) (Transformation|GetDistanceTo (Variables|Default|GetPlayerHead)) _maxscreamrange) _maxscreamrange 1e+02 0.0 1.0) :!class /Script/Engine.AudioComponent))))
    (:Is%20Not%20Valid
      (bind _returnvalue (Actor|GetActorOfClass "/Game/FrazierContent/Entity/Head/BP_HeadCharacter.BP_HeadCharacter_C"))
      (Variables|Default|SetPlayerHead _returnvalue))))

(event Collision|EventHit
  (params (MyComp :type Primitive%20Component%20Object%20Reference) (Other :type Actor%20Object%20Reference) (OtherComp :type Primitive%20Component%20Object%20Reference) (bSelfMoved :type Boolean) (HitLocation :type Vector :default "0, 0, 0") (HitNormal :type Vector :default "0, 0, 0") (NormalImpulse :type Vector :default "0, 0, 0") (Hit :type Hit%20Result%20Structure%20%28by%20ref%29))
  (Utilities|Casting|CastToBP_RootCharacter Other
    (:then
      (CallFunction|BlowUp :!label _label))
    (:CastFailed
      (Utilities|Casting|CastToBP_HeadCharacter Other
        (:then
          (goto _label))
        (:CastFailed
          (Utilities|Casting|CastToBP_SoildHazard Other)
          (Actor|DestroyActor))))))

(fn ConstructionScript)