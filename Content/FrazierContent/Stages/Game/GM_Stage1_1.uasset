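; Game mode for Stage 1-1 that handles enemy-count progression, opening doors as fishing boats are cleared.
; Its UpdateEnemyCount event counts BP_FishingBoat actors and, when one or none remain, destroys every actor tagged "Door" and prints a debug message.
; The same event then tells every BP_EnemySpawner to run CheckSpawnEnemy, using world-wide actor searches rather than stored references.
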(event EventUpdateEnemyCount
  (Utilities|FlowControl|Sequence
    (:then_0
      (bind _outactors (Actor|GetAllActorsOfClass "/Game/FrazierContent/Entity/Enemies/FishingBoat/BP_FishingBoat.BP_FishingBoat_C"))
      (if (<= (Utilities|Array|Length _outactors) 1)
        (bind _outactors_2 (Actor|GetAllActorswithTag "Door"))
        (for _array_element _outactors_2
          (Actor|DestroyActor _array_element))
        (Development|PrintString "Door Open")))
    (:then_1
      (bind _outactors_3 (Actor|GetAllActorsOfClass "/Game/FrazierContent/Entity/Spawner/BP_EnemySpawner.BP_EnemySpawner_C"))
      (for _array_element_2 _outactors_3
        (Default|CheckSpawnEnemy _array_element_2)))))

(fn ConstructionScript)