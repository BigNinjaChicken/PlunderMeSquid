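; BP_RootCharacter is a character that trails the BP_HeadCharacter, using its AI controller to move toward it whenever the distance exceeds MaxRadius.
; Tick finds and caches the Head actor, then runs that distance check each frame.
; A Move event applies camera-relative movement input to a supplied pawn.
; MeshBobb loops a timeline that moves the mesh up and down on Z.
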(event Custom|MeshBobb
  (Components|Timeline|SetPlayRate (Variables|Default|GetT_Bobb) 0.4)
  (bind _value (Timeline|T_Bobb PlayFromStart)
    (:Update
      (Transformation|SetRelativeLocation (Variables|Character|GetMesh) (Math|Vector|MakeVector 0.0 0.0 (Math|Float|Lerp -9e+01 -6e+01 _value)) false false))
    (:Finished
      (Timeline|T_Bobb PlayFromStart))))

(event Custom|Move
  (params (Pawn :type Pawn%20Object%20Reference) (X :type Float%20%28double-precision%29) (Y :type Float%20%28double-precision%29))
  (bind _followcamera (Variables|Camera|GetFollowCamera))
  (bind _returnvalue (Transformation|GetWorldRotation _followcamera))
  (Pawn|Input|AddMovementInput Pawn (Math|Vector|GetRightVector (Math|Rotator|MakeRotator (.roll _returnvalue) 0.0 (.yaw _returnvalue))) X false)
  (Pawn|Input|AddMovementInput Pawn (Math|Vector|GetForwardVector (Math|Rotator|MakeRotator 0.0 0.0 (.yaw (Transformation|GetWorldRotation _followcamera)))) Y false))

(event EventTick
  (params (DeltaSeconds :type Float%20%28single-precision%29))
  (if (not (Utilities|IsValid (Variables|Default|GetHead)))
    (bind _returnvalue (Actor|GetActorOfClass "/Game/MyContent/Head/BP_HeadCharacter.BP_HeadCharacter_C"))
    (Variables|Default|SetHead _returnvalue)
    (else
      (Utilities|FlowControl|Sequence
        (:then_0
          (if (> (Math|Vector|Distance(Vector) (Transformation|GetActorLocation (Variables|Default|GetHead)) (Transformation|GetActorLocation)) (Variables|Tether|GetMaxRadius))
            (AI|Navigation|MovetoLocation (AI|GetAIController self) (Transformation|GetActorLocation (Variables|Default|GetHead)) (Variables|Tether|GetMaxRadius) true true false true 0)))))))

(fn ConstructionScript)