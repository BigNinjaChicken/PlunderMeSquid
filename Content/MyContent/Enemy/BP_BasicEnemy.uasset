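; BP_BasicEnemy is an enemy that fires BP_Canon actors toward the BP_HeadCharacter.
; Tick runs Setup, which finds and caches the head character, then refreshes both actors' locations.
; ShootEvent spawns the projectile ahead of the enemy along the look-at direction, raised vertically, while a slowed Cooldown timeline re-enables CanShoot when finished.
; Nothing here calls ShootEvent or reads the delayed Ready flag, and LookAt is unused.
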(event Custom|ShootEvent
  (bind _selflocation (Variables|Default|GetSelfLocation))
  (bind _headlocation (Variables|Default|GetHeadLocation))
  (bind _selflocation_2 (Variables|Default|GetSelfLocation))
  (bind _returnvalue (Math|Rotator|FindLookatRotation _selflocation _headlocation))
  (bind _returnvalue_2 (Math|Vector|GetForwardVector _returnvalue))
  (bind _returnvalue_3 (* _returnvalue_2 5e+01))
  (bind _returnvalue_4 (+ _returnvalue_3 _selflocation_2))
  (Utilities|FlowControl|Sequence
    (:then_0
      (Components|Timeline|SetPlayRate (Variables|Default|GetCooldown) 0.25)
      (Timeline|Cooldown PlayFromStart
        (:Finished
          (Variables|Default|SetCanShoot true))))
    (:then_1
      (Game|SpawnActorfromClass "/Game/MyContent/Enemy/BP_Canon.BP_Canon_C" (Math|Transform|MakeTransform (Math|Vector|MakeVector (.x _returnvalue_4) (.y _returnvalue_4) (+ (.z _returnvalue_4) 6e+01)) "0, 0, 0" "1.000000,1.000000,1.000000") "Undefined" 0 0))))

(event EventTick
  (params (DeltaSeconds :type Float%20%28single-precision%29))
  (Utilities|FlowControl|Sequence
    (:then_0
      (CallFunction|Setup))))

(event EventBeginPlay
  (Utilities|FlowControl|Delay 1.0)
  (Variables|Default|SetReady true))

(fn ConstructionScript)

(fn Setup
  (if (not (Utilities|IsValid (Variables|Default|GetHead)))
    (bind _returnvalue (Actor|GetActorOfClass "/Game/MyContent/Head/BP_HeadCharacter.BP_HeadCharacter_C"))
    (Variables|Default|SetHead _returnvalue)
    (else
      (Utilities|FlowControl|Sequence
        (:then_0
          (Variables|Default|SetSelfLocation (Transformation|GetActorLocation)))
        (:then_1
          (Variables|Default|SetHeadLocation (Transformation|GetActorLocation (Variables|Default|GetHead))))))))